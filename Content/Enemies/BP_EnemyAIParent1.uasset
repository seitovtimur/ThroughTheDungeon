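; Melee enemy AI character that patrols, chases and attacks the player, with a proximity-shown health bar.
; PawnSensing sets the "HasSeenPlayer?" Blackboard key, cleared by a retriggerable delay.
; Attack turns toward the player and plays a random montage; HitDetection damages through a cooldown-gated right-hand sphere trace.
; HitReact applies the player's MaxDamage, heals the player and stops AI logic, resuming after the reaction montage or destroying the enemy on death.
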(event `HitDetection`
  (bind _returnvalue (`SceneComponent.GetSocketLocation` (`self.Mesh`) "RightHand"))
  (if (`self.CanDetectHit`)
    (bind _outhit (`KismetSystemLibrary.SphereTraceSingleForObjects` _returnvalue _returnvalue 50.0 (`|MakeArray` "ObjectTypeQuery3" :!type "EObjectTypeQuery Enum")))
    (bind _asbp_third_person_character (cast `/Game/ThirdPerson/Blueprints/BP_ThirdPersonCharacter` (`.HitActor` (`GameplayStatics.BreakHitResult` _outhit))))
    (`GameplayStatics.ApplyDamage` _asbp_third_person_character 10.0)
    (set `self.CanDetectHit` false)
    (`KismetSystemLibrary.Delay` 1.0)
    (set `self.CanDetectHit` true)))

(event `Hit React`
  (if (not (`self.isDying`))
    (bind _asbp_third_person_character (cast `/Game/ThirdPerson/Blueprints/BP_ThirdPersonCharacter` (`GameplayStatics.GetPlayerCharacter` 0)))
    (`/Engine/EditorBlueprintResources/StandardMacros.IsValid` _asbp_third_person_character
      (:`Is Valid`
        (`/Game/ThirdPerson/Blueprints/BP_ThirdPersonCharacter.Heal` _asbp_third_person_character)
        (bind _output_get (set `self.Health` (- (`self.Health`) (`/Game/ThirdPerson/Blueprints/BP_ThirdPersonCharacter.MaxDamage` _asbp_third_person_character))))
        (`self.Update Health Bar`)
        (`BrainComponent.StopLogic` (`AIController.BrainComponent` (`AIBlueprintHelperLibrary.GetAIController` self)) "Dead")
        (if (<= _output_get 0.0)
          (set `self.isDying` true)
          (`|PlayMontage` (`self.Mesh`) "/Game/Animations/Enemies/Dying.Dying"
            (:`then`
              (`KismetSystemLibrary.Delay` 2.9)
              (`self.K2_DestroyActor`)))
          (else
            (`|PlayMontage` (`self.Mesh`) (select `int` (`KismetMathLibrary.RandomIntegerInRange` 0 2) :`0` "/Game/Animations/Enemies/Hit_1.Hit_1" :`1` "/Game/Animations/Enemies/Hit_2.Hit_2" :`2` "/Game/Animations/Enemies/Hit_3.Hit_3" :!type "AnimMontage Object Reference")
              (:`OnCompleted`
                (`BrainComponent.StartLogic` (`AIController.BrainComponent` (`AIBlueprintHelperLibrary.GetAIController` self)))
                (`BlackboardComponent.SetValueAsBool` (`AIBlueprintHelperLibrary.GetBlackboard` (`AIBlueprintHelperLibrary.GetAIController` self)) "HasSeenPlayer?" true)))))))))

(event `self.ReceiveBeginPlay`
  (bind _healthbar (`self.HealthBar`))
  (bind _asw_aihealth_bar (cast `/Game/Enemies/W_AIHealthBar` (`WidgetComponent.GetWidget` _healthbar)))
  (`/Engine/EditorBlueprintResources/StandardMacros.IsValid` _asw_aihealth_bar
    (:`Is Valid`
      (set `/Game/Enemies/W_AIHealthBar.MaxHealth` (`self.MaxHealth`) _asw_aihealth_bar)
      (`self.Update Health Bar`)
      (`SceneComponent.SetVisibility` _healthbar false false))))

(event `self.PawnSensing.OnSeePawn`
  (params (Pawn :type "Pawn Object Reference"))
  (cast `/Game/ThirdPerson/Blueprints/BP_ThirdPersonCharacter` Pawn)
  (`BlackboardComponent.SetValueAsBool` (`AIBlueprintHelperLibrary.GetBlackboard` (`AIBlueprintHelperLibrary.GetAIController` self)) "HasSeenPlayer?" true)
  (`KismetSystemLibrary.RetriggerableDelay` 5.0)
  (`self.Lose Sight`))

(event `Set Patrol Speed`
  (set `CharacterMovementComponent.MaxWalkSpeed` 250.0 (`self.CharacterMovement`)))

(event `Lose Sight`
  (`BlackboardComponent.SetValueAsBool` (`AIBlueprintHelperLibrary.GetBlackboard` (`AIBlueprintHelperLibrary.GetAIController` self)) "HasSeenPlayer?" false))

(event `Set Chase Speed`
  (set `CharacterMovementComponent.MaxWalkSpeed` 500.0 (`self.CharacterMovement`)))

(event `self.Interaction Zone.OnComponentBeginOverlap`
  (params (OverlappedComponent :type "PrimitiveComponent Object Reference") (OtherActor :type "Actor Object Reference") (OtherComp :type "PrimitiveComponent Object Reference") (OtherBodyIndex :type Integer) (bFromSweep :type Boolean) (SweepResult :type "HitResult Structure (by ref)"))
  (cast `/Game/ThirdPerson/Blueprints/BP_ThirdPersonCharacter` OtherActor)
  (`SceneComponent.SetVisibility` (`self.HealthBar`) true false))

(event `self.Interaction Zone.OnComponentEndOverlap`
  (params (OverlappedComponent :type "PrimitiveComponent Object Reference") (OtherActor :type "Actor Object Reference") (OtherComp :type "PrimitiveComponent Object Reference") (OtherBodyIndex :type Integer))
  (cast `/Game/ThirdPerson/Blueprints/BP_ThirdPersonCharacter` OtherActor)
  (`SceneComponent.SetVisibility` (`self.HealthBar`) false false))

(fn `Attack`
  (returns (AnimationDuration :type "Float (double-precision)"))
  (`self.K2_SetActorRotation` (`KismetMathLibrary.RLerp` (`self.K2_GetActorRotation`) (`KismetMathLibrary.FindLookAtRotation` (`self.K2_GetActorLocation`) (`self.K2_GetActorLocation` (`GameplayStatics.GetPlayerCharacter` 0)))))
  (bind _returnvalue (`self.PlayAnimMontage` (select `int` (`KismetMathLibrary.RandomIntegerInRange` 0 2) :`0` "/Game/Animations/Enemies/MeleeAttack_1.MeleeAttack_1" :`1` "/Game/Animations/Enemies/MeleeAttack_2.MeleeAttack_2" :`2` "/Game/Animations/Enemies/MeleeAttack_3.MeleeAttack_3" :!type "AnimMontage Object Reference")))
  (return _returnvalue))

(fn `Update Health Bar`
  (bind _asw_aihealth_bar (cast `/Game/Enemies/W_AIHealthBar` (`WidgetComponent.GetWidget` (`self.HealthBar`))))
  (`/Engine/EditorBlueprintResources/StandardMacros.IsValid` _asw_aihealth_bar
    (:`Is Valid`
      (set `/Game/Enemies/W_AIHealthBar.Health` (`self.Health`) _asw_aihealth_bar)
      (return))))

(fn `UserConstructionScript`)