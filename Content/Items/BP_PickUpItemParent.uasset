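; Base pickup item actor that toggles an interaction prompt widget as overlaps begin and end on its interaction area.
; Interaction sends class, icon and stack size to the player via interface, then destroys the actor, provided W_Inventory has room or a matching stack can take another.
; Impulse events push the mesh away from the player or up and out of a chest.
; AddEffect is a placeholder that only prints.
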(event `/Game/Inventory/PickUpItem_Interface.AddEffect`
  (`KismetSystemLibrary.PrintString` "No Effect Yet"))

(event `/Game/Inventory/PickUpItem_Interface.InteractWithPickUpItem`
  (bind _returnvalue (`GameplayStatics.GetPlayerCharacter` 0))
  (if (`KismetSystemLibrary.DoesImplementInterface` _returnvalue "/Game/Inventory/PickUpItem_Interface.PickUpItem_Interface_C")
    (if (not (`KismetMathLibrary.ClassIsChildOf` (`GameplayStatics.GetObjectClass` _returnvalue)))
      (bind _foundwidgets (`WidgetBlueprintLibrary.GetAllWidgetsOfClass` "/Game/Widgets/Inventory/W_Inventory.W_Inventory_C" false))
      (if (< (`/Game/Widgets/Inventory/W_Inventory.InventorySize` (`|GetArrayItem` _foundwidgets)) 7)
        (message `/Game/Inventory/PickUpItem_Interface.PickUpItem` (`GameplayStatics.GetPlayerCharacter` 0) (`self.ItemClass`) (`self.ItemIcon`) (`self.StackSize`) :!label _label)
        (`self.K2_DestroyActor`)
        (elif (> (`self.StackSize`) 1)
          (bind _foundwidgets_2 (`WidgetBlueprintLibrary.GetAllWidgetsOfClass` "/Game/Widgets/Inventory/W_Inventory.W_Inventory_C" false))
          (for _array_element (`PanelWidget.GetAllChildren` (`/Game/Widgets/Inventory/W_Inventory.InventoryBox` (`|GetArrayItem` _foundwidgets_2)))
            (bind (_itemclass _currentstackamount _maxstackamount) (message `/Game/Inventory/PickUpItem_Interface.GetPickUpItemData` _array_element))
            (if (== _itemclass (`self.ItemClass`))
              (if (<= (+ _currentstackamount 1) _maxstackamount)
                (set `self.IsItemAdded` true)
                (break))))
          (if (`self.IsItemAdded`)
            (goto _label)))))))

(event `self.ReceiveBeginPlay`
  (bind _asw_interaction_prompt (cast `/Game/Widgets/ItemInteraction/W_InteractionPrompt` (`WidgetComponent.GetWidget` (`self.Widget`))))
  (set `/Game/Widgets/ItemInteraction/W_InteractionPrompt.Actor` self _asw_interaction_prompt))

(event `/Game/Inventory/PickUpItem_Interface.PushPickUpItemAway`
  (bind _returnvalue (`KismetMathLibrary.GetForwardVector` (`self.K2_GetActorRotation` (`GameplayStatics.GetPlayerPawn` 0))))
  (`PrimitiveComponent.AddVelocityChangeImpulseAtLocation` (`self.StaticMesh`) (* _returnvalue 250.0) (+ (* _returnvalue (15.0 0.0 0.0)) (`self.K2_GetActorLocation`)) "None"))

(event `/Game/Inventory/PickUpItem_Interface.PushItemFromChest`
  (bind _returnvalue (+ (`KismetMathLibrary.GetForwardVector` (`self.K2_GetActorRotation`)) (0.0 0.0 1.0)))
  (`PrimitiveComponent.AddVelocityChangeImpulseAtLocation` (`self.StaticMesh`) (* _returnvalue 150.0) (+ (* _returnvalue (15.0 0.0 15.0)) (`self.K2_GetActorLocation`)) "None"))

(event `self.Interaction Area.OnComponentBeginOverlap`
  (params (OverlappedComponent :type "PrimitiveComponent Object Reference") (OtherActor :type "Actor Object Reference") (OtherComp :type "PrimitiveComponent Object Reference") (OtherBodyIndex :type Integer) (bFromSweep :type Boolean) (SweepResult :type "HitResult Structure (by ref)"))
  (`SceneComponent.SetVisibility` (`self.Widget`) true false))

(event `self.Interaction Area.OnComponentEndOverlap`
  (params (OverlappedComponent :type "PrimitiveComponent Object Reference") (OtherActor :type "Actor Object Reference") (OtherComp :type "PrimitiveComponent Object Reference") (OtherBodyIndex :type Integer))
  (`SceneComponent.SetVisibility` (`self.Widget`) false false))

(fn `GetPickUpItemData`
  (returns (ItemClass :type "Actor Class Reference") (CurrentStackAmount :type Integer) (MaxStackAmount :type Integer))
  (return null 0 0))

(fn `UserConstructionScript`)