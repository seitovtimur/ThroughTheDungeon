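; BP_Chest is a loot chest that opens when the third-person character overlaps its trigger and drops a random artifact.
; An aura effect and sound run from BeginPlay.
; On overlap it plays the opening animation, swaps effects after a short delay, changes the sound and destroys the trigger.
; A downward debug-drawn trace places the artifact above the floor; RandomInteger(5) never selects the sixth artifact class.
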(event `self.ReceiveBeginPlay`
  (bind _returnvalue (`GameplayStatics.SpawnSoundAtLocation` "/Game/Sounds/S_ChestAura_Cue.S_ChestAura_Cue" (`self.K2_GetActorLocation`) (struct) 1.0 1.0 0.0 "/Game/Sounds/Chest_Aura.Chest_Aura" null))
  (set `self.ChestSound` _returnvalue)
  (`ActorComponent.Activate` (`self.NS_ChestAura`) false))

(event `Drop Loot`
  (bind _returnvalue (`self.K2_GetActorLocation`))
  (`AudioComponent.SetSound` (`self.ChestSound`) "/Game/Sounds/SFX/S_ChestOpen.S_ChestOpen")
  (set `self.isOpened` true)
  (bind _outhit (`KismetSystemLibrary.LineTraceSingle` _returnvalue (- _returnvalue (0.0 0.0 250.0)) "TraceTypeQuery1" false (`|MakeArray` (`GameplayStatics.GetPlayerCharacter` 0) :!type "Actor Object Reference") "ForDuration" true (struct :`R` 1.0 :`A` 1.0) (struct :`G` 1.0 :`A` 1.0) 2.0))
  (bind _returnvalue_2 (`|SpawnActorFromClass` (select `int` (`KismetMathLibrary.RandomInteger` 5) :`0` "/Game/Items/BP_Artifact1.BP_Artifact1_C" :`1` "/Game/Items/BP_Artifact2.BP_Artifact2_C" :`2` "/Game/Items/BP_Artifact3.BP_Artifact3_C" :`3` "/Game/Items/BP_Artifact4.BP_Artifact4_C" :`4` "/Game/Items/BP_Artifact5.BP_Artifact5_C" :`5` "/Game/Items/BP_Artifact6.BP_Artifact6_C" :!type "Actor Class Reference") (`KismetMathLibrary.MakeTransform` (+ (`.Location` (`GameplayStatics.BreakHitResult` _outhit)) (0.0 0.0 70.0)) (`self.K2_GetActorRotation`)) "Undefined" "MultiplyWithRoot" null null))
  (message `/Game/Inventory/PickUpItem_Interface.PushItemFromChest` _returnvalue_2))

(event `self.OpenTriggerBox.OnComponentBeginOverlap`
  (params (OverlappedComponent :type "PrimitiveComponent Object Reference") (OtherActor :type "Actor Object Reference") (OtherComp :type "PrimitiveComponent Object Reference") (OtherBodyIndex :type Integer) (bFromSweep :type Boolean) (SweepResult :type "HitResult Structure (by ref)"))
  (cast `/Game/ThirdPerson/Blueprints/BP_ThirdPersonCharacter` OtherActor)
  (`SkeletalMeshComponent.PlayAnimation` (`self.Chest`) "/Game/Meshes/Chest/Chest_Anim_Armature_ArmatureAction.Chest_Anim_Armature_ArmatureAction" false)
  (`KismetSystemLibrary.Delay` 0.7)
  (`ActorComponent.Deactivate` (`self.NS_ChestAura`))
  (`ActorComponent.Activate` (`self.Niagara`) false)
  (`self.Drop Loot`)
  (`ActorComponent.K2_DestroyComponent` (`self.OpenTriggerBox`)))

(fn `UserConstructionScript`)